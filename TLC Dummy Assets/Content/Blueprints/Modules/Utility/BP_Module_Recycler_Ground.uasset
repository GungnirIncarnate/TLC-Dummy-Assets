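; BP_Module_Recycler_Ground is a utility module Blueprint, named as the ground variant of the recycler.
; Its event graph holds only disabled placeholder events, and its construction script just calls the parent.
; Functions for consumption, remainder, door opening, timeline and switch toggling have empty bodies here, so the file shows no recycling logic of its own.
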(fn `GetConsumptions`)

(fn `GetRemainder`)

(fn `IsConsumptionDynamic`)

(fn `OnSwitchToggleState`)

(fn `OpenDoor`)

(fn `Timeline__FinishedFunc`)

(fn `Timeline__UpdateFunc`)

(fn `UpdateConsumption`)

(fn `UserConstructionScript`
  (`parent.UserConstructionScript`))