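; BP_Inventory_PlayerBox is an interactive inventory container Blueprint, apparently a player storage box with a lid, icon and name text.
; It adds no logic of its own: its event nodes are disabled placeholders and its construction script only calls the parent.
; The functions for lid animation, text widget, icon material and post-load name updates are empty here, which suggests the behaviour lives in a parent class.
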(fn `FixAttachments`)

(fn `HasVisibleIcon`)

(fn `InitTextWidget`)

(fn `LidOpen__FinishedFunc`)

(fn `LidOpen__UpdateFunc`)

(fn `OnInventoryIconChanged_Event`)

(fn `OnInventoryNameUpdated_Event_0`)

(fn `OnLoaded_5E998ADC42BCD31F6A0815A54CD26DA0`)

(fn `OnLoaded_EFB79EC3412EF2776CFAF59FDA446AD2`)

(fn `PlayCloseAnim`)

(fn `PlayOpenAnim`)

(fn `PostLoadUpdateName`)

(fn `UpdateIconMaterial`)

(fn `UpdateTextWidget`)

(fn `UserConstructionScript`
  (`parent.UserConstructionScript`))