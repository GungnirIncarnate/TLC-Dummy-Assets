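; BP_Rocket_Functional is a rocket actor whose function names cover fueling, pods, doors, interaction, persistence and the launch and landing sequence.
; Every listed function body is empty except the construction script, which only calls its parent.
; The event graph holds only disabled placeholder events, so this file adds no visible logic of its own.
; Names point to three timeline-driven fuel hatches, electricity, oxygen and methane modules, pod sockets, and reward handling.
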(fn `CanBeInteractedBy`)

(fn `CanInteractFuelHatch`)

(fn `DoCommitteePackageExchange`)

(fn `DoLaunchPlayback`)

(fn `GatherComponents`)

(fn `GetActorsInsideRocket`)

(fn `GetDataAssetComponent`)

(fn `GetDoorInteractText`)

(fn `GetFuelHatchInteractText`)

(fn `GetFuelHatchResourceType`)

(fn `GetFuelModuleComponent`)

(fn `GetFuelProgress`)

(fn `GetGrabText`)

(fn `GetInteractCrosshair`)

(fn `GetInteractIndices`)

(fn `GetInteractiveProvidedActions`)

(fn `GetInteractiveProvidedGrabActions`)

(fn `GetInteractText`)

(fn `GetInventoryComponent`)

(fn `GetItemsInsideRocket`)

(fn `GetLazarusPod`)

(fn `GetNumFuelHatches`)

(fn `GetNumOccupiedPodSlots`)

(fn `GetOverrideZoneId`)

(fn `GetOwnedPersistentActorComponent`)

(fn `GetOwningPlayerState`)

(fn `GetPodSocketComponent`)

(fn `GetScanText`)

(fn `GetStateComponent`)

(fn `GetUnloadedActorClass`)

(fn `HasAnyChanges`)

(fn `HasBeenLaunched`)

(fn `HasCustomData`)

(fn `HasEmptyPods`)

(fn `HasLoosePods`)

(fn `HasPower`)

(fn `InteractAction`)

(fn `InteractActionPartial`)

(fn `InteractGetInventory`)

(fn `InteractWithGrab`)

(fn `IsAllFuelHatchesClosed`)

(fn `IsDoorOpen`)

(fn `IsDoorPartId`)

(fn `IsFuelHatchCableAttached`)

(fn `IsFuelHatchOpen`)

(fn `IsHatchPartId`)

(fn `IsPodAttached`)

(fn `IsSnapSocketPlugged`)

(fn `MarkHumansLaunched`)

(fn `MarkPodLaunched`)

(fn `MoneyWorth`)

(fn `OnAbortLaunchSequence`)

(fn `OnActorAttached`)

(fn `OnCapsuleActorSpawned_Event`)

(fn `OnCountdownSecondChanged_Event`)

(fn `OnCustomDataLoad`)

(fn `OnCustomDataSave`)

(fn `OnDestroyUnloadedActor`)

(fn `OnLanded_Event`)

(fn `OnLanding_Event`)

(fn `OnLaunched`)

(fn `OnLaunched_Event`)

(fn `OnModuleElectricityChanged`)

(fn `OnModuleMethaneChanged`)

(fn `OnModuleOxygenChanged`)

(fn `OnModuleValueChanged`)

(fn `OnPersistentActorPostLoad`)

(fn `OnPersistentActorPrepareSave`)

(fn `OnPersistentActorPreSave`)

(fn `OnPersistentSubsystemPostLoad`)

(fn `OnPersistentSubsystemPreSave`)

(fn `OnPersistentTranformReset`)

(fn `OnRequestLaunch_Event`)

(fn `OnRequestLaunchSequence`)

(fn `OnSnapSocketConnectionChanged`)

(fn `OnSpawnUnloadedActor`)

(fn `OnStateCompleted`)

(fn `OnStateProgressChanged_Event`)

(fn `PersistComponentTranform`)

(fn `PersistTranform`)

(fn `PlayDoorLockedSound`)

(fn `PlayDoorSound`)

(fn `PlayerInteraction`)

(fn `PlayerInteractionRelease`)

(fn `PlayFuelHatchInterruptedSound`)

(fn `PlayFuelHatchSound`)

(fn `ProcessRocketContent`)

(fn `QueueReward`)

(fn `SetDoorLocation`)

(fn `SetDoorTimeline`)

(fn `SetFuelHatchTime_01`)

(fn `SetFuelHatchTime_02`)

(fn `SetFuelHatchTime_03`)

(fn `SetHatchRotation`)

(fn `SetRocketTopVisible`)

(fn `SetupInteractiveState`)

(fn `ShouldIgnoreVisiblityTrace`)

(fn `TickPodSocketState`)

(fn `Timeline__FinishedFunc`)

(fn `Timeline__UpdateFunc`)

(fn `TL_OpenFuelHatch_01__FinishedFunc`)

(fn `TL_OpenFuelHatch_01__UpdateFunc`)

(fn `TL_OpenFuelHatch_02__FinishedFunc`)

(fn `TL_OpenFuelHatch_02__UpdateFunc`)

(fn `TL_OpenFuelHatch_03__FinishedFunc`)

(fn `TL_OpenFuelHatch_03__UpdateFunc`)

(fn `ToggleDoor`)

(fn `ToggleFuelHatch_01`)

(fn `ToggleFuelHatch_02`)

(fn `ToggleFuelHatch_03`)

(fn `ToggleInteractions`)

(fn `UpdateLightState`)

(fn `UserConstructionScript`
  (`parent.UserConstructionScript`))